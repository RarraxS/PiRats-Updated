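; World interaction manager that drives player-centered foliage interaction through a Niagara system and the MPC_Foliage material parameter collection.
; BeginPlay derives the interactor max distance and sends grid and response settings to Niagara, and grid dimensions to the collection.
; Each tick flattens registered components' locations, radii and velocities into Niagara arrays.
; It also feeds current and previous player locations to both, with optional element-count debug printing.
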(event EventBeginPlay
  (bind _interactionniagarasystem (Variables|Default|GetInteractionNiagaraSystem))
  (bind _numcellsresolution (Variables|Settings|GetNumCellsResolution))
  (bind _interactionareaworldsize (Variables|Settings|GetInteractionAreaWorldSize))
  (bind _returnvalue (/ _interactionareaworldsize _numcellsresolution))
  (Variables|Other|SetPlayerPawn (Game|Player|GetPlayerPawn 0))
  (if (Variables|Settings|GetEnableInteractorMaxDistanceOverride)
    (Variables|Other|SetInteractorMaxDistance (Variables|Settings|GetInteractorMaxDistanceOverride))
    (else
      (Variables|Other|SetInteractorMaxDistance (* (Variables|Settings|GetInteractionAreaWorldSize) 0.5))))
  ;[1 1 1] Set constant variables for Niagara interaction system
  (Niagara|SetNiagaraVariable(Float) _interactionniagarasystem "WorldSize" (Variables|Settings|GetInteractionAreaWorldSize))
  (Class|NiagaraComponent|SetVariableInt _interactionniagarasystem "NumCells" (Variables|Settings|GetNumCellsResolution))
  (Niagara|SetNiagaraVariable(Float) _interactionniagarasystem "InteractStrength" (Variables|Settings|GetInteractStrength))
  (Niagara|SetNiagaraVariable(Float) _interactionniagarasystem "SquashMin" (Variables|Settings|GetSquashMin))
  (Niagara|SetNiagaraVariable(Float) _interactionniagarasystem "SquashMax" (Variables|Settings|GetSquashMax))
  (Niagara|SetNiagaraVariable(Float) _interactionniagarasystem "DirectionResistance" (Variables|Settings|GetDirectionResistance))
  (Niagara|SetNiagaraVariable(Float) _interactionniagarasystem "DirectionResistanceBias" (Variables|Settings|GetDirectionResistanceBias))
  (Niagara|SetNiagaraVariable(Float) _interactionniagarasystem "RecoverRate" (Variables|Settings|GetRecoverRate))
  (Niagara|SetNiagaraVariable(Float) _interactionniagarasystem "EdgeFalloffSize" (- 0.5 (/ (Variables|Settings|GetEdgeFalloffSize) 2.0)))
  (Niagara|SetNiagaraVariable(Float) _interactionniagarasystem "EdgeFalloffRate" (Variables|Settings|GetEdgeFalloffRate))
  (Niagara|SetNiagaraVariable(Float) _interactionniagarasystem "InteractionSpread" (Variables|Settings|GetInteractionSpread))
  (Class|NiagaraComponent|SetVariableInt _interactionniagarasystem "SafeMaxInteractingElements" (Variables|Settings|GetSafeMaxInteractingElements))
  (Niagara|SetNiagaraVariable(Float) _interactionniagarasystem "CellSize" _returnvalue)
  ;[1 1 1] Set MPC variables
  (Rendering|Material|SetScalarParameterValue "/Game/AeonStylized/Shared/Materials/MPC/MPC_Foliage.MPC_Foliage" "Interaction World Size" (Variables|Settings|GetInteractionAreaWorldSize) :!class /Script/Engine.KismetMaterialLibrary)
  (Rendering|Material|SetScalarParameterValue "/Game/AeonStylized/Shared/Materials/MPC/MPC_Foliage.MPC_Foliage" "Interaction Num Cells" (Math|Conversions|ToFloat(Integer) (Variables|Settings|GetNumCellsResolution)) :!class /Script/Engine.KismetMaterialLibrary)
  (Rendering|Material|SetScalarParameterValue "/Game/AeonStylized/Shared/Materials/MPC/MPC_Foliage.MPC_Foliage" "Interaction Cell Size" _returnvalue :!class /Script/Engine.KismetMaterialLibrary))

(event EventTick
  (params (DeltaSeconds :type Float%20%28single-precision%29))
  (bind _interactionniagarasystem (Variables|Default|GetInteractionNiagaraSystem))
  ;[1 1 1] Make this actor tied to the player location
  (Variables|Other|SetPlayerLocation (Transformation|GetActorLocation (Variables|Other|GetPlayerPawn)))
  (Utilities|FlowControl|Sequence
    (:then_0
      ;[1 1 1] Clear old array data
      (Utilities|Array|Clear (Variables|Other|GetInteractionArrayA))
      (Utilities|Array|Clear (Variables|Other|GetInteractionArrayB))
      (Utilities|Array|Clear (Variables|Other|GetInteractionArrayC))
      (if (Variables|Settings|GetEnableInteractions)
        ;[1 1 1] Create arrays for location, radius, and velocity of all interacting components
        (bind _result (Utilities|Set|ToArray (Variables|Other|GetInteractingActorComponents)))
        (for _array_element _result
          (for (_array_element_2 _array_index) (Variables|/Game/AeonStylized/NatureVol1/Blueprints/AC_Interactor.AC_Interactor_C|GetInteractionLocationArray _array_element)
            (Utilities|Array|Add (Variables|Other|GetInteractionArrayA) _array_element_2)
            (Utilities|Array|Add (Variables|Other|GetInteractionArrayB) (Utilities|Array|Get(acopy) (Variables|/Game/AeonStylized/NatureVol1/Blueprints/AC_Interactor.AC_Interactor_C|GetInteractionRadiiArray _array_element) _array_index))
            (Utilities|Array|Add (Variables|Other|GetInteractionArrayC) (Utilities|Array|Get(acopy) (Variables|/Game/AeonStylized/NatureVol1/Blueprints/AC_Interactor.AC_Interactor_C|GetInteractionVelocityArray _array_element) _array_index))))))
    (:then_1
      ;[1 1 1] Update Niagara variables with new array data
      (Class|NiagaraDataInterfaceArrayFunctionLibrary|SetNiagaraArrayVector _interactionniagarasystem "InteractionArrayA" (Variables|Other|GetInteractionArrayA))
      (Class|NiagaraDataInterfaceArrayFunctionLibrary|SetNiagaraArrayVector _interactionniagarasystem "InteractionArrayB" (Variables|Other|GetInteractionArrayB))
      (Class|NiagaraDataInterfaceArrayFunctionLibrary|SetNiagaraArrayVector _interactionniagarasystem "InteractionArrayC" (Variables|Other|GetInteractionArrayC))
      (Niagara|SetNiagaraVariable(Vector3) _interactionniagarasystem "PlayerLocation" (Variables|Other|GetPlayerLocation))
      (Niagara|SetNiagaraVariable(Vector3) _interactionniagarasystem "PlayerLocationLast" (Variables|Other|GetPlayerLocationLast))
      ;[1 1 1] Update MPC variables with player location
      (Rendering|Material|SetVectorParameterValue "/Game/AeonStylized/Shared/Materials/MPC/MPC_Foliage.MPC_Foliage" "Player Location" (Math|Conversions|ToLinearColor(Vector) (Variables|Other|GetPlayerLocation)) :!class /Script/Engine.KismetMaterialLibrary)
      (Rendering|Material|SetVectorParameterValue "/Game/AeonStylized/Shared/Materials/MPC/MPC_Foliage.MPC_Foliage" "Player Location Last" (Math|Conversions|ToLinearColor(Vector) (Variables|Other|GetPlayerLocationLast)) :!class /Script/Engine.KismetMaterialLibrary)
      (Variables|Other|SetPlayerLocationLast (Variables|Other|GetPlayerLocation)))
    (:then_2
      (if (Variables|Settings|GetPrintTotalInteractingElements)
        (Development|PrintString (Utilities|String|Append "Total Foliage Interacting Elements: " (Utilities|String|ToString(Integer) (Utilities|Array|Length (Variables|Other|GetInteractionArrayA)))) true true "(R=0.000000,G=0.660000,B=1.000000,A=1.000000)" 0.0)))))

(fn ConstructionScript)