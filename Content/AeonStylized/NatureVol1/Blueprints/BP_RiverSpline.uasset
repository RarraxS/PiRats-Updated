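; River spline Blueprint that lays a river mesh along a spline as a chain of deformed spline mesh segments.
; The construction script derives segment count from mesh length and X scale, evens the spacing, and clamps tangents to that spacing, with configurable material, width and collision.
; Custom primitive data passes segment index, UV scales and start/end fade settings to the material, and is reapplied on BeginPlay.
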(event EventBeginPlay
  (for (_array_element _array_index) (Variables|Default|GetSplineMeshArray)
    (CallFunction|SetCustomPrimitiveData _array_element _array_index)))

(fn ConstructionScript
  (bind _river_mesh (Variables|Default|GetRiver%20Mesh))
  (bind _scale (Variables|MeshSize|GetScale))
  (bind _returnvalue (Math|Vector2D|MakeVector2D (.y _scale) 1.0))
  (bind _returnvalue_2 (StaticMesh|GetBoundingBox _river_mesh))
  (Utilities|Array|Clear (Variables|Default|GetSplineMeshArray))
  (Variables|Default|SetSpacing (* (.x (- (.max _returnvalue_2) (.min _returnvalue_2))) (.x (Variables|MeshSize|GetScale))))
  (bind _output_get (Variables|Default|SetNumSegments (Math|Float|Round (/ (Spline|GetSplineLength (Variables|Default|GetSpline)) (Variables|Default|GetSpacing)))))
  (Variables|Default|SetSpacing (/ (Spline|GetSplineLength (Variables|Default|GetSpline)) _output_get))
  (for _index (range 0 (- (Variables|Default|GetNumSegments) 1))
    (Variables|Default|SetIndex _index)
    (bind _returnvalue_3 (AddComponent|AddSplineMeshComponent false))
    (Utilities|Array|Add (Variables|Default|GetSplineMeshArray) _returnvalue_3)
    (Components|StaticMesh|SetStaticMesh _returnvalue_3 (Variables|Default|GetRiver%20Mesh))
    (Rendering|Material|SetMaterial _returnvalue_3 0 (Variables|Default|GetMaterial%20Instance))
    (SplineMesh|SetForwardAxis _returnvalue_3 "X" true)
    (SplineMesh|SetStartandEnd _returnvalue_3 (.Position (CallFunction|GetSplineData (Variables|Default|GetIndex))) (.Tangent (CallFunction|GetSplineData (Variables|Default|GetIndex))) (.Position (CallFunction|GetSplineData (Variables|Default|GetIndex) 1)) (.Tangent (CallFunction|GetSplineData (Variables|Default|GetIndex) 1)) true :!class /Script/Engine.SplineMeshComponent)
    (SplineMesh|SetStartScale _returnvalue_3 _returnvalue true :!class /Script/Engine.SplineMeshComponent)
    (SplineMesh|SetEndScale _returnvalue_3 _returnvalue true :!class /Script/Engine.SplineMeshComponent)
    (Collision|SetCollisionEnabled _returnvalue_3 (Variables|MeshCollision|GetCollision%20Type))
    (CallFunction|SetCustomPrimitiveData _returnvalue_3 (Variables|Default|GetIndex))))

(fn GetSplineData
  (params (Index :type Integer) (Index%20Offset :type Integer))
  (bind _returnvalue (+ Index Index%20Offset))
  (bind _spacing (Variables|Default|GetSpacing))
  (bind _spline (Variables|Default|GetSpline))
  (bind _returnvalue_2 (* _returnvalue _spacing))
  (return (Spline|GetLocationatDistanceAlongSpline _spline _returnvalue_2 "Local") (Math|Vector|ClampVectorSize (Spline|GetTangentatDistanceAlongSpline _spline _returnvalue_2 "Local") 0.0 (Variables|Default|GetSpacing))))

(fn SetCustomPrimitiveData
  (params (Input :type Primitive%20Component%20Object%20Reference) (Index :type Integer))
  (Rendering|Material|SetCustomPrimitiveDataFloat Input 0 (Math|Conversions|ToFloat(Integer) Index))
  (Rendering|Material|SetCustomPrimitiveDataFloat Input 10 (Variables|UVs|GetU%20Scale))
  (Rendering|Material|SetCustomPrimitiveDataFloat Input 11 (Variables|UVs|GetV%20Scale))
  (if (== Index 0)
    (Rendering|Material|SetCustomPrimitiveDataFloat Input 1 1.0)
    (Rendering|Material|SetCustomPrimitiveDataFloat Input 2 (Variables|StartandEndFading|GetRiver%20Start%20Fade%20Bias))
    (Rendering|Material|SetCustomPrimitiveDataFloat Input 3 (Variables|StartAndEndFading|GetRiver%20Start%20Fade%20Strength))
    (elif (== Index (- (Variables|Default|GetNumSegments) 1))
      (Rendering|Material|SetCustomPrimitiveDataFloat Input 4 1.0)
      (Rendering|Material|SetCustomPrimitiveDataFloat Input 5 (Variables|StartAndEndFading|GetRiver%20End%20Fade%20Bias))
      (Rendering|Material|SetCustomPrimitiveDataFloat Input 6 (Variables|StartAndEndFading|GetRiver%20End%20Fade%20Strength)))))