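; Actor component that makes its owner an interactor for the level's BP_WorldInteraction actor, disabling itself if none exists.
; While within max distance of the player pawn, it registers in that actor's component set, otherwise it unregisters.
; Each tick it fills location, radius and velocity arrays from skeletal mesh bones or owner-relative spheres, deriving velocity from frame-to-frame movement.
; It supports manual enabling, disabling and debug sphere drawing.
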(event Custom|Manually%20Enable%20Interaction
  ;[1 1 1] Get References to Actors in World
  (Components|Tick|SetComponentTickEnabled true)
  (Variables|Ignore-DoNotModify|SetComponentEnabled true)
  (bind _returnvalue (Actor|GetActorOfClass "/Game/AeonStylized/NatureVol1/Blueprints/BP_WorldInteraction.BP_WorldInteraction_C"))
  (Utilities|IsValid _returnvalue
    (:Is%20Valid
      (Variables|Ignore-DoNotModify|SetWorldInteractionActor _returnvalue)
      (Variables|Ignore-DoNotModify|SetPlayerPawn (Game|Player|GetPlayerPawn 0))
      (Variables|Ignore-DoNotModify|SetOwner (Components|GetOwner))
      (if (Variables|OverrideMaxInteractorDistance|GetEnableInteractorMaxDistanceOverride)
        (Variables|Ignore-DoNotModify|SetInteractorMaxDistance (Variables|OverrideMaxInteractorDistance|GetInteractorMaxDistanceOverride))
        (else
          (Variables|Ignore-DoNotModify|SetInteractorMaxDistance (Variables|/Game/AeonStylized/NatureVol1/Blueprints/BP_WorldInteraction.BP_WorldInteraction_C|GetInteractorMaxDistance (Variables|Ignore-DoNotModify|GetWorldInteractionActor)))))
      (Variables|Ignore-DoNotModify|SetInSet false)
      (if (Variables|BoneMode|GetUseBoneInteractors)
        ;[1 1 1] Set initial location of bones
        (if (Variables|BoneMode|GetGetSkeletalMeshByTag)
          (Variables|Ignore-DoNotModify|SetSkeletalMesh (Utilities|Array|Get(acopy) (Actor|GetComponentsbyTag (Variables|Ignore-DoNotModify|GetOwner) "/Script/Engine.SkeletalMeshComponent" (Variables|BoneMode|GetSkeletalMeshTag))))
          (else
            (Variables|Ignore-DoNotModify|SetSkeletalMesh (Actor|GetComponentbyClass (Variables|Ignore-DoNotModify|GetOwner) "/Script/Engine.SkeletalMeshComponent"))))
        (CallFunction|InitialBoneLocation)
        (else
          ;[1 1 1] Set initial location of simple interactors
          (CallFunction|InitialSimpleLocation))))
    (:Is%20Not%20Valid
      ;;[1 1 1] If no BP_WorldInteraction actor is found in level, disable the tick function to avoid errors
      (Components|Tick|SetComponentTickEnabled false)
      (Variables|Ignore-DoNotModify|SetComponentEnabled false)
      (Development|PrintString "No BP_WorldInteraction actor found in world"))))

(event Custom|Manually%20Disable%20Interaction
  ;[1 1 1] Get References to Actors in World
  (Components|Tick|SetComponentTickEnabled false)
  (Variables|Ignore-DoNotModify|SetComponentEnabled false)
  (CallFunction|RemovefromInteractorsSet))

(event EventBeginPlay
  ;[1 1 1] Get References to Actors in World
  (bind _returnvalue (Actor|GetActorOfClass "/Game/AeonStylized/NatureVol1/Blueprints/BP_WorldInteraction.BP_WorldInteraction_C"))
  (Utilities|IsValid _returnvalue
    (:Is%20Valid
      (Variables|Ignore-DoNotModify|SetWorldInteractionActor _returnvalue)
      (Variables|Ignore-DoNotModify|SetPlayerPawn (Game|Player|GetPlayerPawn 0))
      (Variables|Ignore-DoNotModify|SetOwner (Components|GetOwner))
      (if (Variables|OverrideMaxInteractorDistance|GetEnableInteractorMaxDistanceOverride)
        (Variables|Ignore-DoNotModify|SetInteractorMaxDistance (Variables|OverrideMaxInteractorDistance|GetInteractorMaxDistanceOverride))
        (else
          (Variables|Ignore-DoNotModify|SetInteractorMaxDistance (Variables|/Game/AeonStylized/NatureVol1/Blueprints/BP_WorldInteraction.BP_WorldInteraction_C|GetInteractorMaxDistance (Variables|Ignore-DoNotModify|GetWorldInteractionActor)))))
      (Variables|Ignore-DoNotModify|SetInSet false)
      (if (Variables|BoneMode|GetUseBoneInteractors)
        ;[1 1 1] Set initial location of bones
        (if (Variables|BoneMode|GetGetSkeletalMeshByTag)
          (Variables|Ignore-DoNotModify|SetSkeletalMesh (Utilities|Array|Get(acopy) (Actor|GetComponentsbyTag (Variables|Ignore-DoNotModify|GetOwner) "/Script/Engine.SkeletalMeshComponent" (Variables|BoneMode|GetSkeletalMeshTag))))
          (else
            (Variables|Ignore-DoNotModify|SetSkeletalMesh (Actor|GetComponentbyClass (Variables|Ignore-DoNotModify|GetOwner) "/Script/Engine.SkeletalMeshComponent"))))
        (CallFunction|InitialBoneLocation)
        (else
          ;[1 1 1] Set initial location of simple interactors
          (CallFunction|InitialSimpleLocation))))
    (:Is%20Not%20Valid
      ;;[1 1 1] If no BP_WorldInteraction actor is found in level, disable the tick function to avoid errors
      (Components|Tick|SetComponentTickEnabled false)
      (Variables|Ignore-DoNotModify|SetComponentEnabled false)
      (Development|PrintString "No BP_WorldInteraction actor found in world"))))

(event EventTick
  (params (DeltaSeconds :type Float%20%28single-precision%29))
  (if (< (Math|Vector|Distance(Vector) (Transformation|GetActorLocation (Variables|Ignore-DoNotModify|GetPlayerPawn)) (Transformation|GetActorLocation (Variables|Ignore-DoNotModify|GetOwner))) (Variables|Ignore-DoNotModify|GetInteractorMaxDistance))
    ;[1 1 1] Check if AC Interactor is/isn't in the array of interacting actor components in BP_WorldInteraction
    (if (Variables|Ignore-DoNotModify|GetInSet)
      _
      (else
        (Utilities|Set|Add (Variables|/Game/AeonStylized/NatureVol1/Blueprints/BP_WorldInteraction.BP_WorldInteraction_C|GetInteractingActorComponents (Variables|Ignore-DoNotModify|GetWorldInteractionActor)) self)
        (if (Variables|BoneMode|GetUseBoneInteractors)
          (CallFunction|InitialBoneLocation)
          (else
            (CallFunction|InitialSimpleLocation)))
        (Variables|Ignore-DoNotModify|SetInSet true)))
    (if (Variables|BoneMode|GetUseBoneInteractors)
      ;[1 1 1] Set array data for bone interactors
      (for (_array_element _array_index) (Variables|BoneMode|GetBoneInteractors)
        (CallFunction|SetArrayData _array_index (Transformation|GetSocketLocation (Variables|Ignore-DoNotModify|GetSkeletalMesh) (.BoneName (Utilities|Struct|BreakBoneInteractorStruct _array_element))) (.InteractionRadius (Utilities|Struct|BreakBoneInteractorStruct _array_element)) (.InteractionVelocityStrength (Utilities|Struct|BreakBoneInteractorStruct _array_element)) (.InteractionVelocityMinimum (Utilities|Struct|BreakBoneInteractorStruct _array_element))))
      (else
        ;[1 1 1] Set array data for simple interactors
        (for (_array_element_2 _array_index_2) (Variables|SimpleMode|GetSimpleInteractors)
          (CallFunction|SetArrayData _array_index_2 (Math|Transform|TransformLocation (Transformation|GetActorTransform (Variables|Ignore-DoNotModify|GetOwner)) (.InteractionSphereLocation (Utilities|Struct|BreakSimpleInteractorStruct _array_element_2))) (.InteractionRadius (Utilities|Struct|BreakSimpleInteractorStruct _array_element_2)) (.InteractionVelocityStrength (Utilities|Struct|BreakSimpleInteractorStruct _array_element_2)) (.InteractionVelocityMinimum (Utilities|Struct|BreakSimpleInteractorStruct _array_element_2))))))
    (else
      ;[1 1 1] Remove actor component from interacting actors component set it's if far away from player
      (CallFunction|RemovefromInteractorsSet))))

(event EventEndPlay
  (params (EndPlayReason :type EEndPlayReason%20Enum :default "Destroyed"))
  ;[1 1 1] Remove actor component from interacting actor component set on end play
  (CallFunction|RemovefromInteractorsSet))

(fn SetArrayData
  (params (Index :type Integer) (Location :type Vector) (Radius :type Float%20%28double-precision%29) (Interaction%20Velocity%20Strength :type Float%20%28double-precision%29) (Interaction%20Velocity%20Minimum :type Float%20%28double-precision%29))
  (Utilities|Array|SetArrayElem (Variables|Ignore-DoNotModify|GetInteractionVelocityArray) Index (* (/ (- Location (Utilities|Array|Get(acopy) (Variables|Ignore-DoNotModify|GetInteractionLocationArray) Index)) (Utilities|Time|GetWorldDeltaSeconds)) Interaction%20Velocity%20Strength) true)
  (Utilities|Array|SetArrayElem (Variables|Ignore-DoNotModify|GetInteractionLocationArray) Index Location true)
  (Utilities|Array|SetArrayElem (Variables|Ignore-DoNotModify|GetInteractionRadiiArray) Index (Math|Vector|MakeVector Radius Interaction%20Velocity%20Minimum 0.0) true)
  (if (Variables|Visualize|GetVisualizeInteractionSpheres)
    (Rendering|Debug|DrawDebugSphere Location Radius 16 "(R=1.000000,G=1.000000,B=1.000000,A=1.000000)" 0.0)))

(fn InitialBoneLocation
  (for (_array_element _array_index) (Variables|BoneMode|GetBoneInteractors)
    (Utilities|Array|SetArrayElem (Variables|Ignore-DoNotModify|GetInteractionLocationArray) _array_index (Transformation|GetSocketLocation (Variables|Ignore-DoNotModify|GetSkeletalMesh) (.BoneName (Utilities|Struct|BreakBoneInteractorStruct _array_element))) true)))

(fn InitialSimpleLocation
  (for (_array_element _array_index) (Variables|SimpleMode|GetSimpleInteractors)
    (Utilities|Array|SetArrayElem (Variables|Ignore-DoNotModify|GetInteractionLocationArray) _array_index (Math|Transform|TransformLocation (Transformation|GetActorTransform (Variables|Ignore-DoNotModify|GetOwner)) (.InteractionSphereLocation (Utilities|Struct|BreakSimpleInteractorStruct _array_element))) true)))

(fn RemovefromInteractorsSet
  (if (Variables|Ignore-DoNotModify|GetInSet)
    (Utilities|Set|Remove (Variables|/Game/AeonStylized/NatureVol1/Blueprints/BP_WorldInteraction.BP_WorldInteraction_C|GetInteractingActorComponents (Variables|Ignore-DoNotModify|GetWorldInteractionActor)) self)
    (Variables|Ignore-DoNotModify|SetInSet false)))