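; Door Blueprint that opens only once its linked key has been collected.
; On Interact, it casts the Key reference to Key_BP and checks GotKey.
; If set, the RotacionPuerta timeline lerps the static mesh's relative yaw to swing it slightly; otherwise it prints a missing-key message ("Falta llave").
; BeginPlay caches the player as Character_BP, though the door logic never uses it.
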(event EventBeginPlay
  (bind _ascharacter_bp (Utilities|Casting|CastToCharacter_BP (Game|GetPlayerCharacter 0)))
  (Variables|Default|SetAs%20Character%20BP _ascharacter_bp))

(event Collision|EventActorBeginOverlap
  (params (OtherActor :type Actor%20Object%20Reference)))

(event EventTick
  (params (DeltaSeconds :type Float%20%28single-precision%29)))

(event EventInteract
  (bind _askey_bp (Utilities|Casting|CastToKey_BP (Variables|Default|Getkey)))
  (if (Variables|/Game/BluePrints/Key_BP.Key_BP_C|GetGotKey _askey_bp)
    (bind _z (Timeline|RotacionPuerta Play)
      (:Update
        (Transformation|SetRelativeRotation (Variables|Default|GetStaticMesh) (Math|Rotator|MakeRotator 0.0 0.0 (Math|Float|Lerp 0.0 -1e+01 _z)) false false)))
    (else
      (Development|PrintText "Falta llave"))))

(fn ConstructionScript)