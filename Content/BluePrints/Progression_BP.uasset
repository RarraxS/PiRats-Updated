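; Progression actor that shows the item-collecting UI to the player when the first item has been delivered but the second has not.
; Every Tick it checks its ItemsDelivered flags and whether the player Character_BP's CollectingItemsUI still equals that character's null placeholder variable.
; If so, it creates a Collecting_Items_UI widget, adds it to the viewport, stores it on the character and builds it for stage 2.
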(event EventBeginPlay)

(event Collision|EventActorBeginOverlap
  (params (OtherActor :type Actor%20Object%20Reference)))

(event EventTick
  (params (DeltaSeconds :type Float%20%28single-precision%29))
  (bind _items_delivered (Variables|Default|GetItems%20Delivered))
  (bind _ascharacter_bp (Utilities|Casting|CastToCharacter_BP (Game|GetPlayerCharacter 0)))
  (if (and (== (Variables|/Game/BluePrints/Character_BP.Character_BP_C|GetCollecting%20Items%20UI _ascharacter_bp) (Variables|/Game/BluePrints/Character_BP.Character_BP_C|GetNull%20Collecting%20Items%20UI _ascharacter_bp)) (and (Utilities|Array|Get(acopy) _items_delivered) (not (Utilities|Array|Get(acopy) _items_delivered 1))))
    (bind _returnvalue (UserInterface|CreateWidget "/Game/UserInterface/Collecting_Items_UI.Collecting_Items_UI_C" (Game|GetPlayerController 0)))
    (UserInterface|Viewport|AddtoViewport _returnvalue 0)
    (bind _output_get (Variables|/Game/BluePrints/Character_BP.Character_BP_C|SetCollecting%20Items%20UI _ascharacter_bp _returnvalue))
    ;[1 1 1] Set the image of the pices
    (Default|BuildUI _output_get "/Game/UserInterface/IMAGENES_UI/Imagenes1/2.2")))

(fn ConstructionScript)