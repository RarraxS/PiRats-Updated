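; Rotatable statue actor that advances through four quarter-turn yaw states relative to its Base each time it receives Interact.
; Interact selects the next angle, prints it and sets HasToMove, which blocks further input and lets Tick call CalculateRotation.
; CalculateRotation lerps Statue yaw from Base yaw, not its current yaw, and clears the flag when yaw equals that same lerped value.
; RotateStatue is an uncalled helper.
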(event EventBeginPlay
  (Variables|Default|SetRotation%20State 0)
  (Variables|Default|SetRotation 0)
  (Variables|Default|SetTime%20Remaining 0.0)
  (Variables|Default|SetHas%20To%20Move false))

(event Collision|EventActorBeginOverlap
  (params (OtherActor :type Actor%20Object%20Reference)))

(event EventTick
  (params (DeltaSeconds :type Float%20%28single-precision%29))
  (if (Variables|Default|GetHas%20To%20Move)
    (CallFunction|CalculateRotation (Variables|Default|GetRotation) DeltaSeconds)))

(event EventInteract
  (if (not (Variables|Default|GetHas%20To%20Move))
    (switch int (+ 1 (Variables|Default|GetRotation%20State))
      (:Default
        (Variables|Default|SetRotation%20State 0)
        (Variables|Default|SetRotation 0))
      (:0
        (Variables|Default|SetRotation 0)
        (Variables|Default|SetRotation%20State (+ 1 (Variables|Default|GetRotation%20State)) :!label _label))
      (:1
        (Variables|Default|SetRotation 90)
        (goto _label))
      (:2
        (Variables|Default|SetRotation 180)
        (goto _label))
      (:3
        (Variables|Default|SetRotation 270)
        (goto _label)))
    (Variables|Default|SetHas%20To%20Move true)
    (Development|PrintString (Utilities|String|ToString(Integer) (Variables|Default|GetRotation)))))

(fn ConstructionScript)

(fn CalculateRotation
  (params (Rotation%20To%20Apply :type Integer) (Delta%20Time :type Float%20%28double-precision%29))
  (bind _statue (Variables|Default|GetStatue))
  (bind _base (Variables|Default|GetBase))
  (bind _returnvalue (Transformation|GetWorldRotation _statue))
  (bind _returnvalue_2 (Transformation|GetWorldRotation _base))
  (LocalVariables|SetLocal%20Rotation Rotation%20To%20Apply)
  (if (<= (Variables|Default|GetTime%20Remaining) (Variables|Default|GetTime%20To%20Rotate))
    (bind _output_get (Variables|Default|SetTime%20Remaining (+ Delta%20Time (Variables|Default|GetTime%20Remaining))))
    (Transformation|SetWorldRotation _statue (Math|Rotator|MakeRotator (.roll _returnvalue) (.pitch _returnvalue) (Math|Float|Lerp (.yaw _returnvalue_2) (+ (.yaw _returnvalue_2) (LocalVariables|GetLocal%20Rotation)) (/ _output_get (Variables|Default|GetTime%20To%20Rotate)))) false false)
    (if (== (.yaw _returnvalue) (Math|Float|Lerp (.yaw _returnvalue_2) (+ (.yaw _returnvalue_2) (LocalVariables|GetLocal%20Rotation)) (/ _output_get (Variables|Default|GetTime%20To%20Rotate))))
      (Variables|Default|SetHas%20To%20Move false)
      (Variables|Default|SetTime%20Remaining 0.0))))

(fn RotateStatue
  (bind _statue (Variables|Default|GetStatue))
  (bind _returnvalue (Transformation|GetWorldRotation _statue))
  (Transformation|SetWorldRotation _statue (Math|Rotator|MakeRotator (.roll _returnvalue) (.pitch _returnvalue) (Math|Float|Lerp (.yaw (Transformation|GetWorldRotation (Variables|Default|GetBase))) 0.0 (/ (Variables|Default|GetTime%20Remaining) (Variables|Default|GetTime%20To%20Rotate)))) false false))