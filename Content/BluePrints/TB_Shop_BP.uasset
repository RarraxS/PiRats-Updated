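; TB_Shop_BP is a shop drop-off actor that turns collectable boxes into player points.
; Shortly after BeginPlay it finds and caches the top-level Player_UI widget.
; When a Collectable_Box_BP overlaps its collision component, it adds that box's Points through the UI widget, then destroys the box.
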(event OnComponentBeginOverlap(CollisionComponent)
  (params (OverlappedComponent :type Primitive%20Component%20Object%20Reference) (OtherActor :type Actor%20Object%20Reference) (OtherComp :type Primitive%20Component%20Object%20Reference) (OtherBodyIndex :type Integer) (bFromSweep :type Boolean) (SweepResult :type Hit%20Result%20Structure%20%28by%20ref%29))
  ;[1 1 1] Passes the information of how many points have to be added to the player
  (bind _ascollectable_box_bp (Utilities|Casting|CastToCollectable_Box_BP OtherActor))
  (Utilities|FlowControl|Sequence
    (:then_0
      (Default|AddPoints (Variables|Default|GetPlayer%20UI) (Variables|/Game/BluePrints/Collectable_Box_BP.Collectable_Box_BP_C|GetPoints _ascollectable_box_bp)))
    (:then_1
      (Actor|DestroyActor _ascollectable_box_bp))))

(event EventBeginPlay
  (Utilities|FlowControl|Delay 0.1)
  (bind _foundwidgets (Widget|GetAllWidgetsOfClass "/Game/UserInterface/Player_UI.Player_UI_C" true))
  (Variables|Default|SetPlayer%20UI (Utilities|Array|Get(acopy) _foundwidgets)))

(event EventTick
  (params (DeltaSeconds :type Float%20%28single-precision%29)))

(event Collision|EventActorBeginOverlap
  (params (OtherActor :type Actor%20Object%20Reference)))

(fn ConstructionScript)