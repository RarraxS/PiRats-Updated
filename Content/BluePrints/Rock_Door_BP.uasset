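; Rock door Blueprint that slides its Rock component vertically over a set time once its MoveDoor flag is true.
; Tick accumulates elapsed time up to TimeToOpen and lerps the rock's world Z from the actor's own height to the Target actor's height, keeping X and Y.
; Nothing in this graph sets MoveDoor, and the movement has no reverse.
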(event EventBeginPlay
  (Variables|Default|SetTime%20Remaining 0.0))

(event Collision|EventActorBeginOverlap
  (params (OtherActor :type Actor%20Object%20Reference)))

(event EventTick
  (params (DeltaSeconds :type Float%20%28single-precision%29))
  (bind _rock (Variables|Default|GetRock))
  (bind _returnvalue (Transformation|GetWorldLocation _rock))
  (if (and (<= (Variables|Default|GetTime%20Remaining) (Variables|Default|GetTime%20To%20Open)) (Variables|Default|GetMove%20Door))
    (bind _output_get (Variables|Default|SetTime%20Remaining (+ (Variables|Default|GetTime%20Remaining) DeltaSeconds)))
    (Transformation|SetWorldLocation _rock (Math|Vector|MakeVector (.x _returnvalue) (.y _returnvalue) (Math|Float|Lerp (.z (Transformation|GetActorLocation)) (.z (Transformation|GetActorLocation (Variables|Default|GetTarget))) (/ _output_get (Variables|Default|GetTime%20To%20Open)))) false false)))

(fn ConstructionScript)