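; Item-collection tracker that is meant to move a rock, apparently a door, once all pieces are collected.
; GetAPiece writes the notifying item's ItemsCollected slot, then adds true entries to a never-reset count and sets MoveRock upon reaching the array length.
; Tick ignores MoveRock, always lerping the rock's current Z toward EndPosition by unclamped TimePassed over TimeToOpenDoor and printing that ratio.
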(event EventBeginPlay)

(event Collision|EventActorBeginOverlap
  (params (OtherActor :type Actor%20Object%20Reference)))

(event EventTick
  (params (DeltaSeconds :type Float%20%28single-precision%29))
  (bind _rock (Variables|Default|GetRock))
  (bind _staticmeshcomponent (Variables|/Script/Engine.StaticMeshActor|GetStaticMeshComponent _rock))
  (bind _returnvalue (Transformation|GetWorldLocation _staticmeshcomponent))
  (if true
    (bind _output_get (Variables|Default|SetTime%20Passed (+ DeltaSeconds (Variables|Default|GetTime%20Passed))))
    (Transformation|SetWorldLocation _staticmeshcomponent (Math|Vector|MakeVector (.x _returnvalue) (.y _returnvalue) (Math|Float|Lerp (.z _returnvalue) (.z (Transformation|GetActorLocation (Variables|Default|GetEnd%20Position))) (/ _output_get (Variables|Default|GetTime%20To%20Open%20Door)))) false false)
    (Development|PrintString (Utilities|String|ToString(Float) (/ _output_get (Variables|Default|GetTime%20To%20Open%20Door))))))

(fn ConstructionScript)

(fn GetAPiece
  (params (Item%20Who%20Notified :type Collectable%20Puzzle%20Item%20BP%20Object%20Reference))
  (bind (_array_element _array_index) (Utilities|Array|ForEachLoopwithBreak (Variables|Default|GetItems) :!label _label)
    (:LoopBody
      (if (== _array_element Item%20Who%20Notified)
        (Utilities|Array|SetArrayElem (Variables|Default|GetItems%20Collected) _array_index false)
        (goto _label Break)))
    (:Completed
      (for _array_element_2 (Variables|Default|GetItems%20Collected)
        (if _array_element_2
          (LocalVariables|SetNumber%20Of%20Items%20Collected (+ (LocalVariables|GetNumber%20Of%20Items%20Collected) 1))))
      (if (>= (LocalVariables|GetNumber%20Of%20Items%20Collected) (Utilities|Array|Length (Variables|Default|GetItems%20Collected)))
        (Variables|Default|SetMove%20Rock true)))))