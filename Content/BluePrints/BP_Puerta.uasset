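; BP_Puerta is a locked door that the player can open and close once they hold the skull key.
; BeginPlay caches the player's Character_BP, and Interact checks its LlaveSkull flag before doing anything.
; A valid interaction sets Abierta, then a FlipFlop alternates playing and reversing the RotacionPuerta timeline, which drives the StaticMesh's relative yaw.
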(event EventBeginPlay
  (bind _ascharacter_bp (Utilities|Casting|CastToCharacter_BP (Game|GetPlayerCharacter 0)))
  (Variables|Default|SetAs%20Character%20BP _ascharacter_bp))

(event Collision|EventActorBeginOverlap
  (params (OtherActor :type Actor%20Object%20Reference)))

(event EventTick
  (params (DeltaSeconds :type Float%20%28single-precision%29)))

(event EventInteract
  (Utilities|FlowControl|Sequence
    (:then_0
      (if (Variables|/Game/BluePrints/Character_BP.Character_BP_C|GetLlaveSkull (Variables|Default|GetAs%20Character%20BP))
        (if (Variables|Default|Getabierta)
          _
          (else
            (Variables|Default|Setabierta true)))
        (Utilities|FlowControl|FlipFlop
          (:A
            (bind _z (Timeline|RotacionPuerta Play)
              (:Update
                (Transformation|SetRelativeRotation (Variables|Default|GetStaticMesh) (Math|Rotator|MakeRotator 0.0 0.0 _z) false false))))
          (:B
            (Timeline|RotacionPuerta Reverse)))))))

(fn ConstructionScript)