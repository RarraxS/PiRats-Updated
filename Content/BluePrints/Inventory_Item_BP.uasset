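; Inventory_Item_BP is a pickup item that the player can store in the Character_BP inventory slots.
; On BeginPlay, it enables gravity and physics only if its static mesh is visible.
; When interacted with while visible, it puts itself into the first slot holding the null item.
; It then hides its mesh and disables physics, collision and gravity, so the actor persists instead of being destroyed.
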(event EventBeginPlay
  (bind _staticmesh (Variables|Default|GetStaticMesh))
  ;[1 1 1] Sets the physics at the beginning of the game
  (if (Variables|/Script/Engine.SceneComponent|GetbVisible (Variables|Default|GetStaticMesh))
    (Physics|SetEnableGravity _staticmesh true)
    (Physics|SetSimulatePhysics _staticmesh true)
    (else
      (Physics|SetEnableGravity _staticmesh false)
      (Physics|SetSimulatePhysics _staticmesh false))))

(event Collision|EventActorBeginOverlap
  (params (OtherActor :type Actor%20Object%20Reference)))

(event EventTick
  (params (DeltaSeconds :type Float%20%28single-precision%29)))

(event EventInteract
  (bind _staticmesh (Variables|Default|GetStaticMesh))
  (if (Variables|/Script/Engine.SceneComponent|GetbVisible (Variables|Default|GetStaticMesh))
    (bind _ascharacter_bp (Utilities|Casting|CastToCharacter_BP (Game|GetPlayerCharacter 0)))
    (bind _output_get (Variables|Default|SetCharacter%20BP _ascharacter_bp))
    (bind (_array_element _array_index) (Utilities|Array|ForEachLoopwithBreak (Variables|/Game/BluePrints/Character_BP.Character_BP_C|GetSlots _output_get) :!label _label)
      (:LoopBody
        (if (== _array_element (Variables|Default|GetNull%20Invetory%20Item))
          (Utilities|Array|SetArrayElem (Variables|/Game/BluePrints/Character_BP.Character_BP_C|GetSlots (Variables|Default|GetCharacter%20BP)) _array_index self)
          (Rendering|SetVisibility _staticmesh false true)
          (Physics|SetSimulatePhysics _staticmesh false)
          (Collision|SetCollisionEnabled _staticmesh "NoCollision")
          (Physics|SetEnableGravity _staticmesh false)
          (goto _label Break))))))

(fn ConstructionScript)