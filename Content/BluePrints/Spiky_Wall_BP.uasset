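; Spiky wall hazard that closes in over time and kills the player on contact.
; Tick slides the Wall along world Y from the actor's position toward a Target actor over TimeToClose seconds, using a timed Lerp.
; When Character_BP overlaps the Box, it calls PlayerDied, zeroes the timer and teleports the wall back to its starting position, so the closing starts over.
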(event OnComponentBeginOverlap(Box)
  (params (OverlappedComponent :type Primitive%20Component%20Object%20Reference) (OtherActor :type Actor%20Object%20Reference) (OtherComp :type Primitive%20Component%20Object%20Reference) (OtherBodyIndex :type Integer) (bFromSweep :type Boolean) (SweepResult :type Hit%20Result%20Structure%20%28by%20ref%29))
  ;[1 1 1] Kills the player when collided
  (bind _ascharacter_bp (Utilities|Casting|CastToCharacter_BP OtherActor))
  (Default|PlayerDied _ascharacter_bp)
  (Variables|Default|SetTime%20Remaining 0.0)
  (Transformation|SetWorldLocation (Variables|Default|GetWall) (Variables|Default|GetInitial%20Position) false true))

(event EventBeginPlay
  (Variables|Default|SetTime%20Remaining 0.0)
  (Variables|Default|SetInitial%20Position (Transformation|GetWorldLocation (Variables|Default|GetWall))))

(event Collision|EventActorBeginOverlap
  (params (OtherActor :type Actor%20Object%20Reference)))

(event EventTick
  (params (DeltaSeconds :type Float%20%28single-precision%29))
  (bind _wall (Variables|Default|GetWall))
  (bind _returnvalue (Transformation|GetWorldLocation _wall))
  (if (<= (Variables|Default|GetTime%20Remaining) (Variables|Default|GetTime%20To%20Close))
    (bind _output_get (Variables|Default|SetTime%20Remaining (+ (Variables|Default|GetTime%20Remaining) DeltaSeconds)))
    (Transformation|SetWorldLocation _wall (Math|Vector|MakeVector (.x _returnvalue) (Math|Float|Lerp (.y (Transformation|GetActorLocation)) (.y (Transformation|GetActorLocation (Variables|Default|GetTarget))) (/ _output_get (Variables|Default|GetTime%20To%20Close))) (.z _returnvalue)) false false)))

(fn ConstructionScript)