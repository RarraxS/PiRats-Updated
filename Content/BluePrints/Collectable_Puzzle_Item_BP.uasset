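; Collectable puzzle piece Actor that the player picks up through an Interact event.
; On BeginPlay it enables gravity and physics only if its mesh is visible, and caches the level's Collecting_Items_Data_BP actor.
; Interact reports the piece to that data actor via GetAPiece, then hides the mesh and disables its physics, gravity and collision instead of destroying it.
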(event EventBeginPlay
  (bind _staticmesh (Variables|Default|GetStaticMesh))
  ;[1 1 1] Sets the physics at the beginning of the game
  (if (Variables|/Script/Engine.SceneComponent|GetbVisible (Variables|Default|GetStaticMesh))
    (Physics|SetEnableGravity _staticmesh true)
    (Physics|SetSimulatePhysics _staticmesh true)
    (else
      (Physics|SetEnableGravity _staticmesh false)
      (Physics|SetSimulatePhysics _staticmesh false)))
  ;[1 1 1] Access the Collecting Items Data BP
  (bind _outactors (Actor|GetAllActorsOfClass "/Game/BluePrints/Collecting_Items_Data_BP.Collecting_Items_Data_BP_C"))
  (Variables|Default|SetData%20Container (Utilities|Array|Get(acopy) _outactors)))

(event Collision|EventActorBeginOverlap
  (params (OtherActor :type Actor%20Object%20Reference)))

(event EventTick
  (params (DeltaSeconds :type Float%20%28single-precision%29)))

(event EventInteract
  (bind _staticmesh (Variables|Default|GetStaticMesh))
  (if (Variables|/Script/Engine.SceneComponent|GetbVisible (Variables|Default|GetStaticMesh))
    (Default|GetAPiece (Variables|Default|GetData%20Container) self)
    (Rendering|SetVisibility _staticmesh false true)
    (Physics|SetSimulatePhysics _staticmesh false)
    (Collision|SetCollisionEnabled _staticmesh "NoCollision")
    (Physics|SetEnableGravity _staticmesh false)))

(fn ConstructionScript)